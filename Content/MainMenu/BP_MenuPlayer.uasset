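; BP_MenuPlayer drives the main menu: its backdrop cinematic, the credits screen and the handoff into gameplay.
; BeginPlay shows the cursor and loops LS_02 from a random start time.
; PlayCinematic clears widgets, locks input, plays LS_01, then opens "Level" on a fixed timer, not on sequence completion.
; Other events toggle credits and show a win widget; menu screen creation is left unconnected.
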(event Custom|PlayCinematic
  (bind _returnvalue (Game|GetPlayerController 0))
  (Input|SetInputModeGameOnly _returnvalue)
  (Variables|/Script/Engine.PlayerController|SetbShowMouseCursor _returnvalue false)
  (Sequencer|Player|Stop (Variables|Default|GetLS_02) :!class /Script/MovieScene.MovieSceneSequencePlayer)
  (Viewport|RemoveAllWidgets)
  (bind _outactor (Sequencer|Player|CreateLevelSequencePlayer "/Game/Cinematics/LS_01.LS_01" (Utilities|Struct|MakeMovieSceneSequencePlaybackSettings false "(Value=0)" 1.0 0.0 false false true true)))
  (Sequencer|Player|Play (Variables|/Script/LevelSequence.LevelSequenceActor|GetSequencePlayer _outactor) :!class /Script/MovieScene.MovieSceneSequencePlayer)
  (Utilities|Time|SetTimerbyEvent (delegate Custom|OpenLevel) 5.0))

(event Custom|OpenLevel
  (Game|OpenLevel(byName) "Level"))

(event Custom|CreditsMenu
  (bind _returnvalue (UserInterface|CreateWidget "/Game/MainMenu/CreditsMenu.CreditsMenu_C"))
  (bind _output_get (Variables|Default|SetCreditMenu _returnvalue))
  (UserInterface|Viewport|AddtoViewport _returnvalue 0))

(event Custom|CreditsClose
  (Widget|RemovefromParent (Variables|Default|GetCreditMenu)))

(event Custom|WinLevel
  (bind _returnvalue (UserInterface|CreateWidget "/Game/Widgets/W_LevelWin.W_LevelWin_C"))
  (UserInterface|Viewport|AddtoViewport _returnvalue 0))

(event EventBeginPlay
  (Input|SetInputModeGameandUI (Game|GetPlayerController 0) 0 "DoNotLock" true)
  (Variables|/Script/Engine.PlayerController|SetbShowMouseCursor (Game|GetPlayerController 0) true)
  (bind _outactor (Sequencer|Player|CreateLevelSequencePlayer "/Game/Cinematics/LS_02.LS_02" (Utilities|Struct|MakeMovieSceneSequencePlaybackSettings true "(Value=0)" 1.0 0.0 true)))
  (Variables|Default|SetLS_02 (Variables|/Script/LevelSequence.LevelSequenceActor|GetSequencePlayer _outactor))
  (Class|MovieSceneSequencePlayer|PlayLooping (Variables|/Script/LevelSequence.LevelSequenceActor|GetSequencePlayer _outactor) -1))

(fn ConstructionScript)