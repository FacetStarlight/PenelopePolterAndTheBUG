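; Tutorial pickup item that ends the tutorial and starts the level when picked up while focused and on its quest stage.
; It wakes the BUG AI, unlocks the tutorial door with a sound, hides itself, then after a short delay starts the clock.
; It then flags the tutorial done and starts music via the game instance, completes the Door_02 quest, makes the clock light flicker and destroys itself.
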(event Custom|StartLevel
  (bind _tutdoor (Variables|Default|GetTutDoor))
  (bind _clocklight (Variables|Default|GetClockLight))
  (Default|Wakeup (Variables|Default|GetBUG))
  (Variables|/Game/Enviroment/Environment_Merged/Door_01_OLD.Door_01_OLD_C|SetLocked _tutdoor false)
  (Audio|PlaySoundatLocation "/Game/Sound/Effects/unlock_Cue.unlock_Cue" (Transformation|GetActorLocation _tutdoor) "0, 0, 0" 1.0 1.0 0.0 0 0 0)
  (Rendering|SetVisibility (Variables|Default|GetMesh) false true)
  (Utilities|FlowControl|Delay 1.0)
  (Default|StartLevel (Variables|Default|GetClock))
  (bind _asgi_ppand_bug (Utilities|Casting|CastToGI_PPandBUG (Game|GetGameInstance)))
  (Variables|/Game/Blueprints/GI_PPandBUG.GI_PPandBUG_C|SethasDoneTutorial _asgi_ppand_bug true)
  (Default|StartMusic _asgi_ppand_bug)
  (bind _returnvalue (Actor|GetActorOfClass "/Game/Enviroment/Environment_Merged/Door_02.Door_02_C"))
  (Default|CompleteQuest _returnvalue)
  (Audio|PlaySound2D "/Game/Sound/Effects/KeySound.KeySound" 1.0 1.0 0.0 0 0)
  (Rendering|Components|Light|SetLightColor (Variables|/Game/Enviroment/Environment_Merged/CeilingLight.CeilingLight_C|GetPointLight _clocklight) "(R=0.614583,G=0.032347,B=0.000000,A=1.000000)" true)
  (Variables|/Game/Enviroment/Environment_Merged/CeilingLight.CeilingLight_C|SetFlicker _clocklight true)
  (Variables|/Game/Enviroment/Environment_Merged/CeilingLight.CeilingLight_C|SetFlickerAmount _clocklight 5e+01)
  (Actor|DestroyActor))

(event EventBeginPlay
  (bind _returnvalue (Actor|GetActorOfClass "/Game/Blueprints/Entities/EvilGhost/BUGAI/AIC_BUG.AIC_BUG_C"))
  (Variables|Default|SetBUG _returnvalue)
  (|CallParentFunction))

(event Collision|EventActorBeginOverlap
  (params (OtherActor :type Actor%20Object%20Reference)))

(event EventTick
  (params (DeltaSeconds :type Float%20%28single-precision%29)))

(fn ConstructionScript
  (|CallParentFunction))

(fn PickupFunction
  (if (Variables|Default|GetisFocused)
    (if (Variables|Default|GetonQuestStage)
      (CallFunction|StartLevel))))