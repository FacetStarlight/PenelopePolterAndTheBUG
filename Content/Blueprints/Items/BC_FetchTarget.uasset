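; BC_FetchTarget is a pickup item that serves as a fetch quest objective, inactive until its quest stage begins.
; It starts with blank interaction text, and Activate shows its Niagara effect, sets the pickup prompt and flags the quest stage.
; PickupFunction fires the Fetched event and destroys the actor only when it is focused and on that stage.
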(event Custom|Activate
  (Rendering|SetVisibility (Variables|Default|GetNiagara) true false)
  (Variables|Default|SetInteractionText "Press 'E' To Pickup")
  (Variables|Default|SetonQuestStage true))

(event EventBeginPlay
  (Variables|Default|SetInteractionText "")
  (|CallParentFunction))

(event Collision|EventActorBeginOverlap
  (params (OtherActor :type Actor%20Object%20Reference)))

(event EventTick
  (params (DeltaSeconds :type Float%20%28single-precision%29)))

(fn ConstructionScript
  (|CallParentFunction))

(fn PickupFunction
  (if (Variables|Default|GetisFocused)
    (if (Variables|Default|GetonQuestStage)
      (Default|CallFetchedEvent)
      (Actor|DestroyActor))))