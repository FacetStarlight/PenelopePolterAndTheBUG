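; BP_InventoryActor is an inventory item held by the ghost hunter player that can be placed into the world.
; On BeginPlay it caches the player pawn as BP_GhostHunter.
; PlaceItem spawns the WorldActor class at a given location and rotation with an interaction prompt, then decrements NumItems.
; When none remain, it removes itself from the player's inventory and HUD hotbar and destroys itself.
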(event Custom|PlaceItem
  (params (Location :type Vector) (Rotation :type Rotator))
  (bind _numitems (Variables|Default|GetnumItems))
  (Game|SpawnActorfromClass (Variables|Default|GetworldActor) (Math|Transform|MakeTransform Location Rotation "1,1,1") "Undefined" 0 "Press 'E' to interact" 0)
  (Math|Integer|DecrementInt _numitems
    (:%20%20
      (if (<= _numitems 0)
        (Utilities|Array|RemoveItem (Variables|/Game/Blueprints/Entities/Ghost_Hunter/BP_GhostHunter.BP_GhostHunter_C|GetInventoryActors (Variables|Default|GetPlayer)) self)
        (Default|RemoveHorbarItem (Variables|/Game/Blueprints/Entities/Ghost_Hunter/BP_GhostHunter.BP_GhostHunter_C|GetmainHud (Variables|Default|GetPlayer)) (Utilities|GetClass self))
        (Actor|DestroyActor)))))

(event EventBeginPlay
  (bind _asbp_ghost_hunter (Utilities|Casting|CastToBP_GhostHunter (Game|Player|GetPlayerPawn 0)))
  (Variables|Default|SetPlayer _asbp_ghost_hunter))

(event Collision|EventActorBeginOverlap
  (params (OtherActor :type Actor%20Object%20Reference)))

(event EventTick
  (params (DeltaSeconds :type Float%20%28single-precision%29)))

(fn ConstructionScript)