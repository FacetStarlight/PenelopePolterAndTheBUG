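; Tablet item Blueprint that lets the player trigger an Animalese-style talking dialogue while standing inside its collision sphere.
; Overlap toggles input and the MetaSound; leaving stops speech and fades out the dialogue widget.
; Interact spawns the dialogue UI and steps through the speech text with a custom delayed-loop macro gated by CanTalk, mapping each character to a MetaSound sound index for babble synced to the delay.
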(event OnComponentBeginOverlap(CollisionSphere)
  (params (OverlappedComponent :type Primitive%20Component%20Object%20Reference) (OtherActor :type Actor%20Object%20Reference) (OtherComp :type Primitive%20Component%20Object%20Reference) (OtherBodyIndex :type Integer) (bFromSweep :type Boolean) (SweepResult :type Hit%20Result%20Structure%20%28by%20ref%29))
  (if (== OtherActor (Game|GetPlayerCharacter 0))
    (Variables|Default|SetCanTalk true)
    (Input|EnableInput (Game|GetPlayerController 0))
    (Audio|Components|Audio|Play (Variables|Default|GetMS_Animalese) 0.0)))

(event OnComponentEndOverlap(CollisionSphere)
  (params (OverlappedComponent :type Primitive%20Component%20Object%20Reference) (OtherActor :type Actor%20Object%20Reference) (OtherComp :type Primitive%20Component%20Object%20Reference) (OtherBodyIndex :type Integer))
  (if (== (Game|GetPlayerCharacter 0) OtherActor)
    (Variables|Default|SetCanTalk false)
    (Input|DisableInput (Game|GetPlayerController 0))
    (Audio|Components|Audio|FadeOut (Variables|Default|GetMS_Animalese) 0.0 0.0 "Linear" :!class /Script/Engine.AudioComponent)
    (Class|AudioParameterInterface|Trigger (Class|AudioComponent|GetParameterInterface (Variables|Default|GetMS_Animalese)) "Stop Speech")
    (bind _fade (Timeline|FadeUI PlayFromStart)
      (:Update
        (Widget|SetRenderOpacity (Variables|Default|GetSpeech%20UI) _fade))
      (:Finished
        (Widget|SetVisibility (Variables|Default|GetSpeech%20UI) "Hidden")))))

(event EventBeginPlay)

(event Input|ActionEvents|InputActionInteract
  (params (Key :type Key%20Structure :default "None"))
  (:Pressed
    ;[1 1 1] Load subtitle widget and display it as typewriter characters
    (bind _returnvalue (UserInterface|CreateWidget "/Game/Blueprints/Dialogue/B_DIalogue.B_DIalogue_C"))
    (bind _output_get (Variables|Default|SetSpeech%20UI _returnvalue))
    (UserInterface|Viewport|AddtoViewport _output_get 0)
    (Default|Initiate (Variables|Default|GetSpeech%20UI))
    (Utilities|FlowControl|Sequence
      (:then_0
        ;[1 1 1] Set the speed the sounds will play
        (Class|AudioParameterInterface|SetFloat (Class|AudioComponent|GetParameterInterface (Variables|Default|GetMS_Animalese)) "Repeat Delay" (Variables|Default|GetDelayDuration)))
      (:then_1
        (bind _array_element (Utilities|ForEachLoopDelayedwithCheck (Utilities|String|GetCharacterArrayfromString (Utilities|String|ToString(Text) (Variables|Default|GetSpeechText))) (Variables|Default|GetDelayDuration))
          (:Loop%20Body
            (if (Utilities|Array|ContainsItem (Variables|Default|GetNonAlphaCharacters) _array_element)
              (Class|AudioParameterInterface|SetInt (Class|AudioComponent|GetParameterInterface (Variables|Default|GetMS_Animalese)) "Sound Selected" 27)
              (else
                (Class|AudioParameterInterface|SetInt (Class|AudioComponent|GetParameterInterface (Variables|Default|GetMS_Animalese)) "Sound Selected" (.Value (Utilities|Map|Find (Variables|Default|GetLetterToInt) _array_element))))))
          (:Completed
            (Class|AudioParameterInterface|SetInt (Class|AudioComponent|GetParameterInterface (Variables|Default|GetMS_Animalese)) "Sound Selected" 26)
            (Class|AudioParameterInterface|Trigger (Class|AudioComponent|GetParameterInterface (Variables|Default|GetMS_Animalese)) "Stop Speech")))))))

(fn ConstructionScript)