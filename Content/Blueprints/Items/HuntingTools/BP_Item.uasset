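; Base world item for the hunting tools that the ghost hunter player can rotate or pick up while it is focused.
; On BeginPlay it binds to the player's action and rotate events.
; Pickup increments the count of a matching inventory actor, or spawns InventoryActor and adds it to the inventory and HUD hotbar, then destroys itself.
; Focus changes call IsFocusedFunction, which is empty here.
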(event Custom|Pickup
  (CallFunction|PickupFunction))

(event Custom|Rotate
  (CallFunction|RotateFunction))

(event Custom|SetIsFocused
  (params (Focused :type Boolean))
  (bind _output_get (Variables|Default|SetisFocused Focused))
  (CallFunction|IsFocusedFunction _output_get))

(event EventBeginPlay
  (bind _asbp_ghost_hunter (Utilities|Casting|CastToBP_GhostHunter (Game|Player|GetPlayerPawn 0)))
  (bind _output_get (Variables|Default|SetplayerRef _asbp_ghost_hunter))
  (EventDispatchers|BindEventtoPerformAction _output_get (delegate Custom|Pickup))
  (EventDispatchers|BindEventtoRotate _output_get (delegate Custom|Rotate)))

(fn ConstructionScript)

(fn PickupFunction
  (bind _playerref (Variables|Default|GetplayerRef))
  (bind _inventoryactors (Variables|/Game/Blueprints/Entities/Ghost_Hunter/BP_GhostHunter.BP_GhostHunter_C|GetInventoryActors _playerref))
  (if (Utilities|IsValidClass (Variables|Default|GetInventoryActor))
    (if (Variables|Default|GetisFocused)
      (Variables|/Game/Blueprints/Entities/Ghost_Hunter/BP_GhostHunter.BP_GhostHunter_C|SetisInteracting _playerref false)
      (if (Utilities|Array|IsNotEmpty _inventoryactors)
        (for _array_element _inventoryactors
          (if (== (Utilities|GetClass _array_element) (Variables|Default|GetInventoryActor))
            (Math|Integer|IncrementInt (Variables|/Game/Blueprints/Items/InventoryActors/BP_InventoryActor.BP_InventoryActor_C|GetnumItems _array_element)
              (:%20%20
                (Variables|Default|SethasItem true)
                (Actor|DestroyActor)))))
        (if (not (Variables|Default|GethasItem))
          (bind _returnvalue (Game|SpawnActorfromClass (Variables|Default|GetInventoryActor) (Math|Transform|MakeTransform "0, 0, 0" "0, 0, 0" "1,1,1") "Undefined" 0 0 :!label _label))
          (Utilities|Array|Add (Variables|/Game/Blueprints/Entities/Ghost_Hunter/BP_GhostHunter.BP_GhostHunter_C|GetInventoryActors (Variables|Default|GetplayerRef)) _returnvalue)
          (Default|AddHorbarItem (Variables|/Game/Blueprints/Entities/Ghost_Hunter/BP_GhostHunter.BP_GhostHunter_C|GetmainHud (Variables|Default|GetplayerRef)) (Variables|Default|GetInventoryActor))
          (Actor|DestroyActor))
        (else
          (goto _label))))))

(fn RotateFunction
  (if (Variables|Default|GetisFocused)
    (Class|Actor|AddActorWorldRotation self "0.000000,15.000000,0.000000")))

(fn IsFocusedFunction
  (params (isFocused :type Boolean)))