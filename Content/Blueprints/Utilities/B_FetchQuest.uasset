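; Ghost fetch quest actor that tracks one request from being heard to item delivery, driven by a stage enum in its Data struct.
; Tick arms the quest while a microphone is nearby; opening the tablet then plays the request and activates the target item.
; Fetching the item advances the stage.
; Player overlap with the box then completes it, notifying the tablet, removing the ghost trigger and progressing either the tutorial item or a door.
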(event OnComponentBeginOverlap(Box)
  (params (OverlappedComponent :type Primitive%20Component%20Object%20Reference) (OtherActor :type Actor%20Object%20Reference) (OtherComp :type Primitive%20Component%20Object%20Reference) (OtherBodyIndex :type Integer) (bFromSweep :type Boolean) (SweepResult :type Hit%20Result%20Structure%20%28by%20ref%29))
  (bind _data (Variables|Default|GetData))
  (bind (_ghosttrigger _itemtofetch _queststage) (Utilities|Struct|BreakS_FetchQuestData _data))
  ;[1 1 1] Deliver target to ghost
  (if (== OtherActor (Game|Player|GetPlayerPawn 0))
    (if (Utilities|Enum|Equal(Enum) _queststage "NewEnumerator3")
      (Utilities|Struct|SetmembersinS_FetchQuestData (Variables|Default|GetData) "NewEnumerator4")
      (Default|QuestDeliveredItem (Variables|Default|GetTablet) (Variables|Default|GetData))
      (if (Actor|ActorHasTag _ghosttrigger "Tut")
        (bind _returnvalue (Actor|GetActorOfClass "/Game/Blueprints/Items/Tutorial_Item.Tutorial_Item_C"))
        (Variables|/Game/Blueprints/Items/HuntingTools/BP_Item.BP_Item_C|SetonQuestStage _returnvalue true)
        (Rendering|SetVisibility (Variables|/Game/Blueprints/Items/Tutorial_Item.Tutorial_Item_C|GetMesh _returnvalue) true false)
        (else
          (bind _returnvalue_2 (Actor|GetActorOfClass "/Game/Enviroment/Environment_Merged/Door_02.Door_02_C"))
          (Default|CompleteQuest _returnvalue_2)))
      (Audio|PlaySound2D "/Game/Sound/Effects/QuestsEnded_Cue.QuestsEnded_Cue" 1.0 1.0 0.0 0 0)
      (Actor|DestroyActor _ghosttrigger)
      (Class|AISenseHearing|ReportNoiseEvent (Transformation|GetActorLocation (Game|Player|GetPlayerPawn 0)) 1.0 0 1.5e+02 "None"))))

(event Custom|TabletToggle_Event
  (bind _data (Variables|Default|GetData))
  (bind (_ghosttrigger _itemtofetch _queststage) (Utilities|Struct|BreakS_FetchQuestData _data))
  ;[1 1 1] Start listening to request when tablet opened
  (if (Variables|/Game/Blueprints/Entities/Ghost_Hunter/BP_GhostHunter.BP_GhostHunter_C|GetHasTabletOpen (stale EventBeginPlay _asbp_ghost_hunter))
    (if (Utilities|Enum|Equal(Enum) _queststage "NewEnumerator1")
      (Utilities|Struct|SetmembersinS_FetchQuestData (Variables|Default|GetData) "NewEnumerator2")
      (Default|QuestRequestHeard (Variables|Default|GetTablet) (Variables|Default|GetData))
      (bind _asbc_fetch_target (Utilities|Casting|CastToBC_FetchTarget _itemtofetch))
      (Default|Activate _asbc_fetch_target))
    (else
      (Default|QuestEndDialogue (Variables|Default|GetTablet)))))

(event Custom|TargetFetched
  ;[1 1 1] Advance quest when item retrieved
  (if (Utilities|Enum|Equal(Enum) (.QuestStage (Utilities|Struct|BreakS_FetchQuestData (Variables|Default|GetData))) "NewEnumerator2")
    (Utilities|Struct|SetmembersinS_FetchQuestData (Variables|Default|GetData) "NewEnumerator3")))

(event EventBeginPlay
  ;[1 1 1] Get tablet reference
  (bind _asbp_ghost_hunter (Utilities|Casting|CastToBP_GhostHunter (Game|Player|GetPlayerPawn 0)))
  (EventDispatchers|BindEventtoTabletToggle _asbp_ghost_hunter (delegate Custom|TabletToggle_Event))
  (bind _returnvalue (Actor|GetActorOfClass "/Game/Blueprints/Items/HuntingTools/BP_Tablet.BP_Tablet_C"))
  (Variables|Default|SetTablet _returnvalue)
  ;[1 1 1] Get fetch target reference
  (bind _asbc_fetch_target (Utilities|Casting|CastToBC_FetchTarget (.ItemToFetch (Utilities|Struct|BreakS_FetchQuestData (Variables|Default|GetData)))))
  (EventDispatchers|BindEventtoFetchedEvent _asbc_fetch_target (delegate Custom|TargetFetched)))

(event EventTick
  (params (DeltaSeconds :type Float%20%28single-precision%29))
  (bind _data (Variables|Default|GetData))
  (bind _queststage (Utilities|Struct|BreakS_FetchQuestData _data))
  ;[1 1 1] Check if microphone is placed near ghost
  (if (or (Utilities|Enum|Equal(Enum) (.QuestStage (Utilities|Struct|BreakS_FetchQuestData (Variables|Default|GetData))) "NewEnumerator0") (Utilities|Enum|Equal(Enum) (.QuestStage (Utilities|Struct|BreakS_FetchQuestData (Variables|Default|GetData))) "NewEnumerator1"))
    (bind _returnvalue (Actor|GetActorOfClass "/Game/Blueprints/Items/HuntingTools/BC_Microphone.BC_Microphone_C"))
    (Utilities|IsValid _returnvalue
      (:Is%20Valid
        (if (<= (Transformation|GetDistanceTo _returnvalue) 5e+02)
          (if (Utilities|Enum|Equal(Enum) _queststage "NewEnumerator0")
            (Utilities|Struct|SetmembersinS_FetchQuestData (Variables|Default|GetData) "NewEnumerator1")
            (Audio|PlaySound2D "/Game/Sound/Effects/QuestStarted_Cue.QuestStarted_Cue" 1.0 1.0 0.0 0 0)
            (Class|AISenseHearing|ReportNoiseEvent (Transformation|GetActorLocation (Game|Player|GetPlayerPawn 0)) 1.0 0 1.5e+02 "None"))
          (else
            (if (Utilities|Enum|Equal(Enum) _queststage "NewEnumerator1") :!label _label
              (Utilities|Struct|SetmembersinS_FetchQuestData (Variables|Default|GetData) "NewEnumerator0")))))
      (:Is%20Not%20Valid
        (goto _label)))))

(fn ConstructionScript)

(fn CheckforMicrophone)