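; Custom pawn sensing component that detects tagged actors within a range and view angle from its own transform.
; A looping timer line-traces toward each tagged actor, accepting I_Detectable hits in range.
; The angle test widens by the target's bounds, so partly visible large targets can count.
; It broadcasts detected actors with distances each pass, and NoTargetsSensed once after losing all, with optional debug drawing.
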(event Custom|BeginSensing
  (bind _returnvalue (Utilities|Time|SetTimerbyEvent (delegate Custom|Sense) (Variables|Default|GetSensingInterval) true))
  (Variables|Default|SetSensingTimerRef _returnvalue))

(event Custom|Sense
  (bind _targets (CallFunction|SenseforTargets (Variables|Default|GetShowDebug)))
  (if (> (Utilities|Array|Length _targets) 0)
    (Default|CallTargetsSensed _targets)
    (Variables|Default|SetCallNoTargets true)
    (if (Variables|Default|GetShowDebug)
      (for _array_element _targets
        (Development|PrintString (Utilities|String|BuildString(Object) (Utilities|String|ToString(Float) (.Distance (Utilities|Struct|BreakS_DetectionResult _array_element))) ": " (.Actor (Utilities|Struct|BreakS_DetectionResult _array_element))))))
    (elif (Variables|Default|GetCallNoTargets)
      (Default|CallNoTargetsSensed)
      (Variables|Default|SetCallNoTargets false))))

(event EventBeginPlay
  (CallFunction|BeginSensing))

(fn SenseforTargets
  (params (ShowDebug :type Boolean))
  (bind _pawnsensingangle (Variables|Default|GetPawnSensingAngle))
  (Utilities|Array|Clear (LocalVariables|GetValidTargets))
  (if ShowDebug
    (if (< (Variables|Default|GetPawnSensingAngle) 1.8e+02)
      (Class|KismetSystemLibrary|DrawDebugConeinDegrees (.location (Transformation|GetWorldTransform)) (Math|Vector|GetForwardVector) (Variables|Default|GetPawnSensingRange) _pawnsensingangle _pawnsensingangle 12 "(R=1.000000,G=1.000000,B=1.000000,A=1.000000)" (Variables|Default|GetSensingInterval) 2.0)
      (else
        (Rendering|Debug|DrawDebugSphere (.location (Transformation|GetWorldTransform)) (Variables|Default|GetPawnSensingRange) 12 "(R=1.000000,G=1.000000,B=1.000000,A=1.000000)" (Variables|Default|GetSensingInterval) 5.0))))
  (bind _outactors (Actor|GetAllActorswithTag (Variables|Default|GetTagToSense)))
  (for _array_element _outactors
    (bind _validtarget (CallFunction|CheckTargetVaildity _array_element))
    (if (Utilities|IsValid (.Actor (Utilities|Struct|BreakS_DetectionResult _validtarget)))
      (Utilities|Array|AddUnique (LocalVariables|GetValidTargets) _validtarget)))
  (return (LocalVariables|GetValidTargets)))

(fn DebugMessage
  (params (DebugMessage :type String))
  (if (Variables|Default|GetShowDebug)
    (Development|PrintString DebugMessage)))

(fn CheckTargetVaildity
  (params (TargetToCheck :type Actor%20Object%20Reference))
  (bind _output_get (LocalVariables|SetCheckedTarget TargetToCheck))
  (if (Utilities|IsValid _output_get)
    (bind (_outhit _returnvalue) (Collision|LineTraceByChannel (Transformation|GetWorldLocation) (Transformation|GetActorLocation (LocalVariables|GetCheckedTarget)) "TraceTypeQuery1" false (Utilities|Array|MakeArray (Components|GetOwner)) "None" true "(R=1.000000,G=0.000000,B=0.000000,A=1.000000)" "(R=0.000000,G=1.000000,B=0.000000,A=1.000000)" 3.0))
    (if _returnvalue
      (LocalVariables|SetCurrentHitResult _outhit)
      (if (Utilities|DoesObjectImplementInterface (.hitactor (LocalVariables|GetCurrentHitResult)) "/Game/Blueprints/Utilities/I_Detectable.I_Detectable_C")
        (if (<= (.distance (LocalVariables|GetCurrentHitResult)) (Variables|Default|GetPawnSensingRange))
          (if (<= (Class|KismetMathLibrary|DegAcos (Math|Vector|DotProduct (Math|Vector|GetForwardVector) (Math|Vector|GetUnitDirection(Vector) (Transformation|GetWorldLocation) (.Origin (Collision|GetActorBounds (LocalVariables|GetCheckedTarget) true false))))) (+ (Variables|Default|GetPawnSensingAngle) (Class|KismetMathLibrary|DegAcos (Math|Vector|DotProduct (Math|Vector|GetUnitDirection(Vector) (Transformation|GetWorldLocation) (.Origin (Collision|GetActorBounds (LocalVariables|GetCheckedTarget) true false))) (Math|Vector|GetUnitDirection(Vector) (Transformation|GetWorldLocation) (- (.Origin (Collision|GetActorBounds (LocalVariables|GetCheckedTarget) true false)) (Math|Vector|MakeVector (Math|Float|Clamp(Float) (.x (.BoxExtent (Collision|GetActorBounds (LocalVariables|GetCheckedTarget) true false))) 1e+01 999.0) (Math|Float|Clamp(Float) (.y (.BoxExtent (Collision|GetActorBounds (LocalVariables|GetCheckedTarget) true false))) 1e+01 999.0) (Math|Float|Clamp(Float) (.z (.BoxExtent (Collision|GetActorBounds (LocalVariables|GetCheckedTarget) true false))) 1e+01 999.0))))))))
            (return (Utilities|Struct|MakeS_DetectionResult (.hitactor (LocalVariables|GetCurrentHitResult)) (.distance (LocalVariables|GetCurrentHitResult))))
            (else
              (CallFunction|DebugMessage "Pawn sensing target out of vision angle")
              (return "")))
          (else
            (CallFunction|DebugMessage "Hit result out of pawn sensing range")
            (return "")))
        (else
          (CallFunction|DebugMessage "Pawn sensing is blocked by object")
          (return "")))
      (else
        (CallFunction|DebugMessage "No hit from custom pawn sensing")
        (return "")))))