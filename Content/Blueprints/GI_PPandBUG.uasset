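; GI_PPandBUG, by its prefix a Game Instance, handles player death and background music.
; KillPlayer plays a death sound, shows the W_death widget with UI-only input, then after a delay plays the LS_Death level sequence.
; It then fades out the widget's blood and opens "Level".
; StartMusic alternates two songs as 2D sounds in an endless loop timed by fixed Delays.
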(event Custom|KillPlayer
  (Audio|PlaySound2D "/Game/Sound/Effects/DeathSound_Cue.DeathSound_Cue" 1.0 1.0 0.0 0 0)
  (bind _returnvalue (UserInterface|CreateWidget "/Game/Widgets/w_death.w_death_C"))
  (bind _output_get (Variables|Default|SetDeathWidget _returnvalue))
  (UserInterface|Viewport|AddtoViewport _output_get 0)
  (Input|SetInputModeUIOnly (Game|GetPlayerController 0) 0 "LockAlways")
  (bind _returnvalue_2 (Sequencer|Player|CreateLevelSequencePlayer "/Game/Cinematics/LS_Death.LS_Death"))
  (Utilities|FlowControl|Delay 2.0)
  (Sequencer|Player|Play _returnvalue_2 :!class /Script/MovieScene.MovieSceneSequencePlayer)
  (Utilities|FlowControl|Delay 3.0)
  (Default|FadeoutBlood (Variables|Default|GetDeathWidget))
  (Utilities|FlowControl|Delay 0.15)
  (Game|OpenLevel(byName) "Level"))

(event Custom|StartMusic
  (Utilities|FlowControl|Delay 3e+01 :!label _label)
  (Audio|PlaySound2D "/Game/Sound/Music/Song01.Song01" 1.0 1.0 0.0 0 0)
  (Utilities|FlowControl|Delay 6e+01)
  (Audio|PlaySound2D "/Game/Sound/Music/Song03.Song03" 1.0 1.0 0.0 0 0)
  (Utilities|FlowControl|Delay 3e+01)
  (goto _label))