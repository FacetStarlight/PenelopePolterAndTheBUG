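; Grandfather clock environment Blueprint that plays a ticking sound and an increasingly unstable chime once the level starts.
; Both sounds are silenced on BeginPlay until the StartLevel event starts them along with the Warp timeline.
; While playing, Tick adds a random offset within plus or minus the timeline's current value to the chime's pitch, making it wander cumulatively.
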(event Custom|StartLevel
  (Utilities|FlowControl|Sequence
    (:then_0
      (bind _newtrack_0 (Timeline|Warp Play)))
    (:then_1
      (Variables|Default|SetisPlaying true)
      (Audio|Components|Audio|Play (Variables|Default|GetWarpedChime) 0.0)
      (Audio|Components|Audio|Play (Variables|Default|GetTickTok) 0.0))))

(event EventBeginPlay
  (Audio|Components|Audio|Stop (Variables|Default|GetWarpedChime))
  (Audio|Components|Audio|Stop (Variables|Default|GetTickTok)))

(event Collision|EventActorBeginOverlap
  (params (OtherActor :type Actor%20Object%20Reference)))

(event EventTick
  (params (DeltaSeconds :type Float%20%28single-precision%29))
  (bind _warpedchime (Variables|Default|GetWarpedChime))
  (if (Variables|Default|GetisPlaying)
    (Audio|Components|Audio|SetPitchMultiplier _warpedchime (+ (Variables|/Script/Engine.AudioComponent|GetPitchMultiplier _warpedchime) (Math|Random|RandomFloatinRange (* (stale Custom|StartLevel _newtrack_0) -1.0) (stale Custom|StartLevel _newtrack_0))))))

(fn ConstructionScript)